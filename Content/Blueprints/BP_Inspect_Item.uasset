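; BP_Inspect_Item is a world item that shows an interact prompt and hands its mesh over when the player interacts with it.
; The construction script applies ItemModel to the RelicInspected mesh component.
; A P_PressFITEM widget is created at BeginPlay, then added to or removed from the viewport as the player character begins or ends overlap.
; InteractItem returns ItemModel and triggers DestroyItem, which destroys the actor after a short delay.
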(event Custom|Destroy%20Item
  (Utilities|FlowControl|Delay 0.2)
  (Actor|DestroyActor))

(event Collision|EventActorBeginOverlap
  (params (OtherActor :type Actor%20Object%20Reference))
  (if (== OtherActor (Game|GetPlayerCharacter 0))
    (UserInterface|Viewport|AddtoViewport (Variables|Default|GetInteract%20Widget) 0)))

(event Collision|EventActorEndOverlap
  (params (OtherActor :type Actor%20Object%20Reference))
  (if (== (Game|GetPlayerCharacter 0) OtherActor)
    (Widget|RemovefromParent (Variables|Default|GetInteract%20Widget))))

(event EventBeginPlay
  (bind _returnvalue (UserInterface|CreateWidget "/Game/Blueprints/P_PressFITEM.P_PressFITEM_C"))
  (Variables|Default|SetInteract%20Widget _returnvalue))

(fn ConstructionScript
  (Components|StaticMesh|SetStaticMesh (Variables|Default|GetRelicInspected) (Variables|Default|GetItemModel)))

(fn InteractItem
  (CallFunction|DestroyItem)
  (return (Variables|Default|GetItemModel)))