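; BP_Knight is an enemy Knight that relays AI perception results to its AIC_Knight controller.
; A successful sense stores the actor, cancels any pending loss timer and updates the controller's target and line-of-sight keys.
; A failed sense clears line of sight at once but delays dropping the target through a short one-shot timer, giving the knight brief memory of it.
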(event OnTargetPerceptionUpdated(AIPerception)
  (params (Actor :type Actor%20Object%20Reference) (Stimulus :type AI%20Stimulus%20Structure))
  (Variables|Default|SetPerceived%20Actor Actor)
  (if (Utilities|Struct|BreakAIStimulus Stimulus)
    (Utilities|Time|ClearandInvalidateTimerbyHandle (Variables|Default|GetTarget%20Lost%20Timer))
    (Default|UpdateTargetActorKey (.AsAIC%20Knight (Utilities|Casting|CastToAIC_Knight (Pawn|GetController))) (Variables|Default|GetPerceived%20Actor))
    (Default|UpdateHasLineOfSightKey (.AsAIC%20Knight (Utilities|Casting|CastToAIC_Knight (Pawn|GetController))) true)
    (else
      (bind _returnvalue (Utilities|Time|SetTimerbyEvent (delegate Custom|Target%20Lost) 5.0))
      (Variables|Default|SetTarget%20Lost%20Timer _returnvalue)
      (Default|UpdateHasLineOfSightKey (.AsAIC%20Knight (Utilities|Casting|CastToAIC_Knight (Pawn|GetController))) false))))

(event Custom|Target%20Lost
  (Variables|Default|SetPerceived%20Actor 0)
  (Default|UpdateTargetActorKey (.AsAIC%20Knight (Utilities|Casting|CastToAIC_Knight (Pawn|GetController)))))

(fn ConstructionScript)